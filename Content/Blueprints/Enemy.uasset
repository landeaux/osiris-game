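; Enemy character that attacks on contact, takes damage, and raises game difficulty as the player kills more of them.
; Its construction script sets hitpoints and walk speed from the EnemySpawnControl game instance.
; Hits play an attack montage and apply damage with a brief cooldown, while damage from other enemies is ignored.
; On death it increments the player's kill count, periodically raising shared health, speed and spawn rate.
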(event `self.ReceiveAnyDamage`
  (params (Damage :type "Float (single-precision)") (DamageType :type "DamageType Object Reference") (InstigatedBy :type "Controller Object Reference") (DamageCauser :type "Actor Object Reference"))
  ;[1 1 1] Kill Enemies and Increase Kill Count
  (cast `/Game/Blueprints/Enemy` DamageCauser
    (:`CastFailed`
      (set `self.Hitpoints` (- (`self.Hitpoints`) Damage))
      (if (<= (`self.Hitpoints`) 0.0)
        (bind _asfirst_person_character (cast `/Game/Blueprints/FirstPersonCharacter` (`GameplayStatics.GetPlayerCharacter` 0)))
        (bind _result (`/Engine/EditorBlueprintResources/StandardMacros.IncrementInt` (`/Game/Blueprints/FirstPersonCharacter.PlayerKills` _asfirst_person_character))
          (:`  `
            (bind _asenemy_spawn_control (cast `/Game/Blueprints/EnemySpawnControl` (`GameplayStatics.GetGameInstance`)))
            (set `self.GameMode` _asenemy_spawn_control)
            (set `/Game/Blueprints/EnemySpawnControl.Player Kills` _result (`self.GameMode`))
            (if (== (mod _result 20) 0)
              (set `/Game/Blueprints/EnemySpawnControl.EnemyHealth` (+ (`/Game/Blueprints/EnemySpawnControl.EnemyHealth` (`self.GameMode`)) 1.0) (`self.GameMode`)))
            (if (== (mod _result 30) 0)
              (set `/Game/Blueprints/EnemySpawnControl.Enemy Speed` (+ (`/Game/Blueprints/EnemySpawnControl.Enemy Speed` (`self.GameMode`)) 100.0) (`self.GameMode`)))
            (if (== (mod _result 40) 0)
              (bind _output_get (set `/Game/Blueprints/EnemySpawnControl.EnemySpawnRate` (- (`/Game/Blueprints/EnemySpawnControl.EnemySpawnRate` (`self.GameMode`)) 0.1) (`self.GameMode`)))
              (if (<= _output_get 0.0)
                (set `/Game/Blueprints/EnemySpawnControl.EnemySpawnRate` 0.1 (`self.GameMode`))))
            (`self.K2_DestroyActor`)))))))

(event `self.ReceiveHit`
  (params (MyComp :type "PrimitiveComponent Object Reference") (Other :type "Actor Object Reference") (OtherComp :type "PrimitiveComponent Object Reference") (bSelfMoved :type Boolean) (HitLocation :type "Vector Structure") (HitNormal :type "Vector Structure") (NormalImpulse :type "Vector Structure") (Hit :type "HitResult Structure (by ref)"))
  ;[1 1 1] Enemy Attack
  (`AnimInstance.Montage_Play` (`SkeletalMeshComponent.GetAnimInstance` (`self.EnemyMesh`)) "/Game/Enemy/Animations/Attack.Attack" 2.0 "MontageLength" 0.0 true)
  (if (not (`self.RecentHit`))
    (`GameplayStatics.ApplyDamage` Other (`self.EnemyDamage`) null self)
    (set `self.RecentHit` true)
    (`KismetSystemLibrary.Delay` 0.2)
    (set `self.RecentHit` false)))

(fn `UserConstructionScript`
  (bind _asenemy_spawn_control (cast `/Game/Blueprints/EnemySpawnControl` (`GameplayStatics.GetGameInstance`)))
  (set `self.Hitpoints` (`/Game/Blueprints/EnemySpawnControl.EnemyHealth` _asenemy_spawn_control))
  (set `CharacterMovementComponent.MaxWalkSpeed` (`/Game/Blueprints/EnemySpawnControl.Enemy Speed` _asenemy_spawn_control) (`self.CharacterMovement`)))